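; Knife actor Blueprint that switches the visibility of two knife components, Knife1 and Knife2, through number key presses.
; Keys 1 and 2 each show their own knife and hide the other, storing the state in a pair of boolean variables.
; Key 3 sets both booleans true and feeds them through a NAND, which hides both knives.
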(event `self.ReceiveBeginPlay`)

(event `Key|One`
  (params (Key :type "Key Structure"))
  (:`Pressed`
    (set `self.Knife1Visible?` true)
    (set `self.Knife2Visible?` false)
    (`SceneComponent.SetVisibility` (`self.Knife1`) (`self.Knife1Visible?`) false)
    (`SceneComponent.SetVisibility` (`self.Knife2`) (`self.Knife2Visible?`) false)))

(event `Key|Two`
  (params (Key :type "Key Structure"))
  (:`Pressed`
    (set `self.Knife2Visible?` true)
    (set `self.Knife1Visible?` false)
    (`SceneComponent.SetVisibility` (`self.Knife2`) (`self.Knife2Visible?`) false)
    (`SceneComponent.SetVisibility` (`self.Knife1`) (`self.Knife1Visible?`) false)))

(event `Key|Three`
  (params (Key :type "Key Structure"))
  (bind _returnvalue (`KismetMathLibrary.BooleanNAND` (`self.Knife1Visible?`) (`self.Knife2Visible?`)))
  (:`Pressed`
    (set `self.Knife1Visible?` true)
    (set `self.Knife2Visible?` true)
    (`SceneComponent.SetVisibility` (`self.Knife1`) _returnvalue false)
    (`SceneComponent.SetVisibility` (`self.Knife2`) _returnvalue false)))

(fn `UserConstructionScript`)